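; BP_Familiar is a player-controlled side-scrolling character that moves along the world X axis and jumps through Enhanced Input.
; BeginPlay registers the IMC_Familiar mapping context and adds a WBP_Overlay HUD to the viewport.
; Move input snaps controller yaw to 0 or 180 based on acceleration direction, then applies rounded movement input.
; Healthdeduction extends the parent's logic by refreshing the overlay's health bar.
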(event Input|EnhancedActionEvents|EnhancedInputActionIA_Move
  (params (ActionValue :type Float%20%28double-precision%29) (ElapsedSeconds :type Float%20%28double-precision%29) (TriggeredSeconds :type Float%20%28double-precision%29) (InputAction :type Input%20Action%20Object%20Reference :default "/Game/Assets/Inputs/InputActions/IA_Move.IA_Move"))
  (FamiliarInput|FlipController)
  (Pawn|Input|AddMovementInput "1.000000,0.000000,0.000000" (Math|Conversions|ToFloat(Integer) (Math|Float|Round ActionValue)) false))

(event Input|EnhancedActionEvents|EnhancedInputActionIA_Jump
  (params (ActionValue :type Boolean) (ElapsedSeconds :type Float%20%28double-precision%29) (TriggeredSeconds :type Float%20%28double-precision%29) (InputAction :type Input%20Action%20Object%20Reference :default "/Game/Assets/Inputs/InputActions/IA_Jump.IA_Jump"))
  (:Started
    (Character|Jump)))

(event EventBeginPlay
  ;[0.15 0.15 0.15 0.5] Added Mapping Context(Reminder this connects to BP to the actual conrtoller
  (FamiliarInput|AddMappingContext)
  (CallFunction|CreateOverlay))

(fn ConstructionScript)

(fn AddMappingContext
  (bind _asplayer_controller (Utilities|Casting|CastToPlayerController (Pawn|GetController)))
  (Input|AddMappingContext (PlayerController|LocalPlayerSubsystems|GetEnhancedInputLocalPlayerSubsystem _asplayer_controller) "/Game/Assets/Inputs/IMC_Familiar.IMC_Familiar" 0 "(bIgnoreAllPressedKeysUntilRelease=True,bForceImmediately=False,bNotifyUserSettings=False)"))

(fn FlipController
  (Math|Float|CompareFloat (.x (Pawn|Components|CharacterMovement|GetCurrentAcceleration (Variables|Character|GetCharacterMovement))) 0.0
    (:>
      (Pawn|SetControlRotation (Pawn|GetController) (Math|Rotator|MakeRotator 0.0 0.0 0.0)))
    (:<
      (Pawn|SetControlRotation (Pawn|GetController) (Math|Rotator|MakeRotator 0.0 0.0 1.8e+02)))))

(fn CreateOverlay
  (bind _returnvalue (UserInterface|CreateWidget "/Game/UI/Overlay/WBP_Overlay.WBP_Overlay_C" (.AsPlayer%20Controller (Utilities|Casting|CastToPlayerController (Pawn|GetController)))))
  (bind _output_get (Variables|Default|SetOverlay _returnvalue))
  (UserInterface|Viewport|AddtoViewport _output_get 0))

(fn Healthdeduction
  (|CallParentFunction)
  (Default|UpdateHeathbar (Variables|/Game/UI/Overlay/WBP_Overlay.WBP_Overlay_C|GetWBP_FamiliarHealthbar (Variables|Default|GetOverlay)) (Variables|Default|GetHealth) (Variables|Default|GetMaxHealth)))