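; Base character Blueprint that provides a box trace for detecting attack hits.
; AttackBoxTrace sweeps a box between the BoxTraceStart and BoxTraceEnd components, with configurable extent, orientation and object types.
; It only visualizes the result so far: it draws the trace, prints the hit component's name and marks the impact point with a debug sphere, without applying damage or checking for a hit.
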(fn ConstructionScript)

(fn AttackBoxTrace
  (bind _outhit (Class|KismetSystemLibrary|BoxTraceSingleforObjects (Transformation|GetWorldLocation (Variables|AttackTrace|GetBoxTraceStart)) (Transformation|GetWorldLocation (Variables|AttackTrace|GetBoxTraceEnd)) (Variables|AttackTrace|GetTraceExtent) (Variables|AttackTrace|GetBox%20Rotation) (Variables|Default|GetTraceObjectTypes) false 0 "ForDuration" true))
  (Development|PrintString (Utilities|GetDisplayName (.HitComponent (Collision|BreakHitResult _outhit))))
  (Rendering|Debug|DrawDebugSphere (.ImpactPoint (Collision|BreakHitResult _outhit)) 15.0 12 "(R=0.310163,G=1.000000,B=0.311908,A=1.000000)" 5.0))