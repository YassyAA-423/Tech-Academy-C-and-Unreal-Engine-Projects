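; BP_WithinReachBox is an overlap trigger that tells a set of spike actors when a player is within reach.
; When an actor implementing BPI_Player begins overlapping, it passes that actor to every entry in SpikeActors through SetTargetMessage.
; When such an actor stops overlapping, it sends the same message with no target, clearing it without checking for other players still inside.
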(event Collision|EventActorEndOverlap
  (params (OtherActor :type Actor%20Object%20Reference))
  (if (Utilities|DoesObjectImplementInterface OtherActor "/Game/Interface/BPI_Player.BPI_Player_C")
    (for _array_element (Variables|Default|GetSpikeActors)
      (Class|BPIEnemy|SetTarget(Message) _array_element))))

(event Collision|EventActorBeginOverlap
  (params (OtherActor :type Actor%20Object%20Reference))
  (if (Utilities|DoesObjectImplementInterface OtherActor "/Game/Interface/BPI_Player.BPI_Player_C")
    (for _array_element (Variables|Default|GetSpikeActors)
      (Class|BPIEnemy|SetTarget(Message) _array_element OtherActor))))

(fn ConstructionScript)