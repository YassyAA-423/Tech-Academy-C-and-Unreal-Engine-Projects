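; Base Blueprint for enemy characters, providing combat targeting, attack and turn-around hooks.
; SetCombatTarget writes the target into the controller's Blackboard under the combat target key, and Attack triggers the attack animation.
; ChangeDirection turns the actor around by combining its rotation with a 180-degree offset.
; Debug sphere draws at several radii around the actor are left unconnected and never run.
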(event EventAttack
  (CallFunction|PlayAttackAnim))

(event EventSetCombatTarget
  (params (CombatTarget :type Actor%20Object%20Reference))
  (AI|Components|Blackboard|SetValueasObject (AI|GetBlackboard (Pawn|GetController)) (Variables|Default|GetCombatTargetBBKeyName) CombatTarget))

(fn ConstructionScript)

(fn ChangeDirection
  (Transformation|SetActorRotation (Math|Rotator|CombineRotators (Transformation|GetActorRotation) "0.000000,180.000000,0.000000")))