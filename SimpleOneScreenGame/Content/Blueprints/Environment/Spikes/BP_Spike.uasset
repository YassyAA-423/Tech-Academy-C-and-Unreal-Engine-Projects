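; BP_Spike is a spike hazard that damages actors touching it.
; Overlap on its Box component runs a Visibility box trace, then applies fixed damage to the overlapping actor without using the trace result.
; A separate AttackBox function traces at StartBox with configurable extent and orientation, but nothing in this Blueprint calls it.
; Tick only forwards to the parent class.
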(event OnComponentBeginOverlap(Box)
  (params (OverlappedComponent :type Primitive%20Component%20Object%20Reference) (OtherActor :type Actor%20Object%20Reference) (OtherComp :type Primitive%20Component%20Object%20Reference) (OtherBodyIndex :type Integer) (bFromSweep :type Boolean) (SweepResult :type Hit%20Result%20Structure%20%28by%20ref%29))
  (Collision|BoxTraceByChannel "0, 0, 0" "0, 0, 0" "0, 0, 0" "0, 0, 0" "TraceTypeQuery1" false 0 "None")
  (Game|Damage|ApplyDamage OtherActor 1.0 0 0))

(event EventBeginPlay
  (|CallParentFunction) ; This node is disabled and will not be called.\nDrag off pins to build functionality.
)

(event Collision|EventActorBeginOverlap
  (params (OtherActor :type Actor%20Object%20Reference))
  (|CallParentFunction OtherActor) ; This node is disabled and will not be called.\nDrag off pins to build functionality.
)

(event EventTick
  (params (DeltaSeconds :type Float%20%28single-precision%29))
  (|CallParentFunction DeltaSeconds))

(fn ConstructionScript
  (|CallParentFunction))

(fn AttackBox
  (bind _startbox (Variables|Attack|GetStartBox))
  (bind _returnvalue (Transformation|GetWorldLocation _startbox))
  (Collision|BoxTraceByChannel _returnvalue _returnvalue (Variables|Attack|GetTraceExtent) (Variables|Attack|GetBox%20Orientation) "TraceTypeQuery1" false 0 "None"))