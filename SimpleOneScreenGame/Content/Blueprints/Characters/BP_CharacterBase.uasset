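; BP_CharacterBase is a PaperZD-animated character base that handles damage, hit reactions and death.
; AnyDamage subtracts damage from clamped Health, plays the Hurt animation override and quits the game when Health reaches zero.
; Each hit also calls LaunchCharacter for knockback, scaling a normalized actor-location difference by KnockBack on X and Z and adding KnockBackHeight for lift.
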(event Game|Damage|EventAnyDamage
  (params (Damage :type Float%20%28single-precision%29) (DamageType :type Damage%20Type%20Object%20Reference) (InstigatedBy :type Controller%20Object%20Reference) (DamageCauser :type Actor%20Object%20Reference))
  (CallFunction|Healthdeduction)
  (CallFunction|PlayHitReactAnim)
  (if (<= (Variables|Default|GetHealth) 0.0)
    (Game|QuitGame 0 "Quit" false)))

(fn ConstructionScript)

(fn PlayHitReactAnim
  (Class|PaperZDAnimInstance|PlayAnimationOverride (Variables|/Script/PaperZD.PaperZDAnimationComponent|GetAnimInstance (Variables|Default|GetPaperZDAnimation)) "/Game/Blueprints/Characters/Familiar/Animation/AnimSequences/Hurt.Hurt" "DefaultSlot" 1.0 0.0)
  (CallFunction|KnockBackEffect))

(fn Healthdeduction
  (Variables|Default|SetHealth (Math|Float|Clamp(Float) (- (Variables|Default|GetHealth) (Variables|Default|GetDamage)) 0.0 (Variables|Default|GetMaxHealth))))

(fn KnockBackEffect
  (bind _returnvalue (Transformation|GetActorLocation))
  (bind _returnvalue_2 (Transformation|GetActorLocation))
  (bind _knockback (Variables|Default|GetKnockBack))
  (bind _returnvalue_3 (- _returnvalue _returnvalue_2))
  (bind _returnvalue_4 (Class|KismetMathLibrary|VectorNormal2D _returnvalue_3 0.0001))
  (bind _returnvalue_5 (* _returnvalue_4 _knockback))
  (Character|LaunchCharacter (Math|Vector|MakeVector (.x _returnvalue_5) 0.0 (+ (.z _returnvalue_5) (Variables|Default|GetKnockBackHeight))) true true))