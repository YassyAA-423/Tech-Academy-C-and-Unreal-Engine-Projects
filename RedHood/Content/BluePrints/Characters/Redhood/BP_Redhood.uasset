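; BP_Redhood is the player character for 2D side-on movement along the X axis, with jumping.
; BeginPlay adds the IMC_Redhood Enhanced Input mapping context to player 0's controller.
; Movement input is rounded so analog sticks act as on/off, then fed to AddMovementInput.
; FlipController turns the sprite by setting control rotation yaw to face the sign of the current X acceleration.
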(event Input|EnhancedActionEvents|EnhancedInputActionIA_Movement
  (params (ActionValue :type Float%20%28double-precision%29) (ElapsedSeconds :type Float%20%28double-precision%29) (TriggeredSeconds :type Float%20%28double-precision%29) (InputAction :type Input%20Action%20Object%20Reference :default "/Game/Assets/Input/InputActions/IA_Movement.IA_Movement"))
  ;[0.15 0.15 0.15 0.5] Handles the Movement of the Player, and flips the Player sprite when they move left.
  (CallFunction|FlipController)
  (Pawn|Input|AddMovementInput "1.000000,0.000000,0.000000" (Math|Conversions|ToFloat(Integer) (Math|Float|Round ActionValue)) false))

(event Input|EnhancedActionEvents|EnhancedInputActionIA_Jumping
  (params (ActionValue :type Boolean) (ElapsedSeconds :type Float%20%28double-precision%29) (TriggeredSeconds :type Float%20%28double-precision%29) (InputAction :type Input%20Action%20Object%20Reference :default "/Game/Assets/Input/InputActions/IA_Jumping.IA_Jumping"))
  (:Started
    (Character|Jump)))

(event EventBeginPlay
  ;[0.1363 0.4176 0.7073 0.5] Input Mapping Context (This connect the IMC to the player)
  (RedhoodInput|AddMappingContext))

(fn ConstructionScript)

(fn AddMappingContext
  (bind _asplayer_controller (Utilities|Casting|CastToPlayerController (Game|GetPlayerController 0)))
  (Input|AddMappingContext (PlayerController|LocalPlayerSubsystems|GetEnhancedInputLocalPlayerSubsystem _asplayer_controller) "/Game/Assets/Input/IMC_Redhood.IMC_Redhood" 0 "(bIgnoreAllPressedKeysUntilRelease=True,bForceImmediately=False,bNotifyUserSettings=False)"))

(fn FlipController
  (Math|Float|CompareFloat (.x (Pawn|Components|CharacterMovement|GetCurrentAcceleration (Variables|Character|GetCharacterMovement))) 0.0
    (:>
      (Pawn|SetControlRotation (Pawn|GetController) (Math|Rotator|MakeRotator 0.0 0.0 0.0)))
    (:<
      (Pawn|SetControlRotation (Pawn|GetController) (Math|Rotator|MakeRotator 0.0 0.0 1.8e+02)))))