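; BP_EnemyPatrolBox is a trigger area that tells its assigned patrol enemies when a player enters or leaves it.
; On overlap begin, an actor implementing BPI_Player is sent as combat target to every entry in the PartrolActors array via SetCombatTargetMessage.
; On overlap end, the same message goes out with an empty target, clearing it for all of them.
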(event Collision|EventActorBeginOverlap
  (params (OtherActor :type Actor%20Object%20Reference))
  (if (Utilities|DoesObjectImplementInterface OtherActor "/Game/BluePrints/Interfaces/BPI_Player.BPI_Player_C")
    (for _array_element (Variables|Default|GetPartrolActors)
      (Class|BPIEnemy|SetCombatTarget(Message) _array_element OtherActor))))

(event Collision|EventActorEndOverlap
  (params (OtherActor :type Actor%20Object%20Reference))
  (if (Utilities|DoesObjectImplementInterface OtherActor "/Game/BluePrints/Interfaces/BPI_Player.BPI_Player_C")
    (for _array_element (Variables|Default|GetPartrolActors)
      (Class|BPIEnemy|SetCombatTarget(Message) _array_element))))

(fn ConstructionScript)